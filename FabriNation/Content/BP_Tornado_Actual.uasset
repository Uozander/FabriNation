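; BP_Tornado_Actual is a roaming tornado hazard that wrecks residential and industrial buildings.
; On BeginPlay it jumps to a random ground position, then teleports along one random horizontal drift vector in a timed loop.
; Midway through its ten-second life it spawns a successor, which relocates itself, creating an endless overlapping chain.
; Capsule overlaps replace buildings with demolished versions, spawned at the building's location for residential but the tornado's for industrial.
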(event OnComponentBeginOverlap(Capsule)
  (params (OverlappedComponent :type Primitive%20Component%20Object%20Reference) (OtherActor :type Actor%20Object%20Reference) (OtherComp :type Primitive%20Component%20Object%20Reference) (OtherBodyIndex :type Integer) (bFromSweep :type Boolean) (SweepResult :type Hit%20Result%20Structure%20%28by%20ref%29))
  (bind _returnvalue (Utilities|GetClass OtherActor))
  (if (== _returnvalue "/Game/BP_Residential.BP_Residential_C")
    (Variables|Default|SetDestruction%20Location (Transformation|GetActorLocation OtherActor))
    (Actor|DestroyActor OtherActor)
    (Game|SpawnActorfromClass "/Game/BP_DEMO_Res.BP_DEMO_Res_C" (Math|Transform|MakeTransform (Variables|Default|GetDestruction%20Location) "0, 0, 0" "1.000000,1.000000,1.000000") "Undefined" "MultiplyWithRoot" 0 0)
    (elif (== _returnvalue "/Game/BP_Industry.BP_Industry_C")
      (Variables|Default|SetDestruction%20Location (Transformation|GetActorLocation))
      (Actor|DestroyActor OtherActor)
      (Game|SpawnActorfromClass "/Game/BP_DEMO_Ind.BP_DEMO_Ind_C" (Math|Transform|MakeTransform (Variables|Default|GetDestruction%20Location) "0, 0, 0" "1.000000,1.000000,1.000000") "Undefined" "MultiplyWithRoot" 0 0))))

(event EventBeginPlay
  (Utilities|FlowControl|Sequence
    (:then_0
      (Transformation|SetActorLocation (Math|Vector|MakeVector (+ (* (Math|Random|RandomFloat) 1e+04) -1.5e+03) (+ (* (Math|Random|RandomFloat) 1e+04) -1.5e+03) -105.0) false false)
      (Utilities|FlowControl|Delay 5.0)
      (Game|SpawnActorfromClass "BP_Tornado_Actual_C" (Transformation|GetActorTransform) "Undefined" "MultiplyWithRoot" 0 0)
      (Utilities|FlowControl|Delay 5.0)
      (Actor|DestroyActor))
    (:then_1
      (Variables|Default|SetNewVar (Math|Vector|MakeVector (* (- (Math|Random|RandomFloat) 0.5) 1e+02) (* (- (Math|Random|RandomFloat) 0.5) 1e+02) 0.0))
      (Transformation|SetActorLocation (+ (Transformation|GetActorLocation) (Variables|Default|GetNewVar)) false true :!label _label)
      (Utilities|FlowControl|Delay 0.05)
      (goto _label))))

(fn ConstructionScript)