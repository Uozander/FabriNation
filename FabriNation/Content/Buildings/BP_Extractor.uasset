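; BP_Extractor is a coal-producing building that drains the player controller's Wealth while it runs.
; From BeginPlay, one timed loop charges Wealth and adds coal to its Ore stock every half second.
; A parallel loop with randomized delay spawns a BP_Truck once the stock reaches a threshold, hands it the Ore and resets the stock.
; Worker and home-spawn events are deprecated stubs, leaving the trace-based SpawnHome residential logic uncalled.
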(event Custom|CE_HomeSpawn
  (params (Citizen :type Actor%20Object%20Reference))
  ;[1 0.2326 0.1771] DEP
)

(event Custom|CE_WorkerUP
  ;[1 0.3012 0.2552] DEP
)

(event EventBeginPlay
  (Utilities|FlowControl|Sequence
    (:then_0
      (bind _asbp_top_down_controller (Utilities|Casting|CastToBP_TopDownController (Game|GetPlayerController 0)))
      (Variables|Default|SetAs%20BP%20Top%20Down%20Controller _asbp_top_down_controller)
      (Utilities|FlowControl|Delay 0.5 :!label _label)
      (Variables|/Game/TopDown/Blueprints/BP_TopDownController.BP_TopDownController_C|SetWealth (Variables|Default|GetAs%20BP%20Top%20Down%20Controller) (- (Variables|/Game/TopDown/Blueprints/BP_TopDownController.BP_TopDownController_C|GetWealth (Variables|Default|GetAs%20BP%20Top%20Down%20Controller)) 48.0))
      (Variables|Default|SetOre (Utilities|Struct|MakeSTCT_Resource (+ (.ore_amount (Variables|Default|GetOre)) 60) "Coal" 1))
      (goto _label))
    (:then_1
      (if (>= (.ore_amount (Variables|Default|GetOre)) 100) :!label _label_2
        (bind _returnvalue (Game|SpawnActorfromClass "/Game/Units/BP_Truck.BP_Truck_C" (Transformation|GetActorTransform) "Undefined" "MultiplyWithRoot" 0 0))
        (Default|CEDeliver _returnvalue (Variables|Default|GetOre))
        (Variables|Default|SetOre (Utilities|Struct|MakeSTCT_Resource 0 "Coal" 1)))
      (Utilities|FlowControl|Delay (+ (* (Math|Random|RandomFloat) 3.0) 4.0))
      (goto _label_2))))

(fn ConstructionScript)

(fn SpawnHome
  (params (Direction :type Vector) (Citizen :type Actor%20Object%20Reference))
  (bind _structure (Variables|Default|GetStructure))
  (bind _returnvalue (Transformation|GetWorldLocation _structure))
  (bind _returnvalue_2 (+ _returnvalue Direction))
  (bind _returnvalue_3 (- _returnvalue_2 "0.000000,0.000000,50.000000"))
  (bind (_outhit _returnvalue_4) (Collision|LineTraceByChannel (+ _returnvalue "0.000000,0.000000,50.000000") _returnvalue_2 "TraceTypeQuery1" false 0 "ForOneFrame"))
  (if _returnvalue_4
    (if (== (Utilities|GetClass (.HitActor (Collision|BreakHitResult _outhit))) "/Game/Buildings/BP_Residential.BP_Residential_C")
      (bind _asbp_residential (Utilities|Casting|CastToBP_Residential (.HitActor (Collision|BreakHitResult _outhit))))
      (if (>= (Variables|/Game/Buildings/BP_Residential.BP_Residential_C|GetLevel _asbp_residential) 5)
        (Actor|DestroyActor Citizen)
        (else
          (Default|CETierUp _asbp_residential Citizen)))
      (else
        (Actor|DestroyActor Citizen)))
    (else
      (Game|SpawnActorfromClass "/Game/Buildings/BP_Residential.BP_Residential_C" (Math|Transform|MakeTransform _returnvalue_3 "0, 0, 0" "1.000000,1.000000,1.000000") "Undefined" "MultiplyWithRoot" 0 0)
      (bind _asbp_citizen (Utilities|Casting|CastToBP_Citizen Citizen))
      (Variables|/Game/Units/BP_Citizen.BP_Citizen_C|SetHome%20Location _asbp_citizen _returnvalue_3))))