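; BP_AI is a townsperson character that gets a random head colour at BeginPlay.
; Capsule hits occasionally switch its NavModifier to an obstacle area for a short delay.
; Unconnected graphs, which never run, hold a road speed boost and a commuter routine: pick random industry work, drain food and medical needs, and lerp by Timeline between work and home, grocery or clinic.
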(event OnComponentHit(CapsuleComponent)
  (params (HitComponent :type Primitive%20Component%20Object%20Reference) (OtherActor :type Actor%20Object%20Reference) (OtherComp :type Primitive%20Component%20Object%20Reference) (NormalImpulse :type Vector :default "0, 0, 0") (Hit :type Hit%20Result%20Structure%20%28by%20ref%29))
  (bind _navmodifier (Variables|Default|GetNavModifier))
  (if (== (Variables|/Script/NavigationSystem.NavModifierComponent|GetAreaClass _navmodifier) 0)
    (if (>= (Math|Random|RandomFloat) 0.99)
      (Class|NavModifierComponent|SetAreaClass _navmodifier "/Script/NavigationSystem.NavArea_Obstacle")
      (Utilities|FlowControl|Delay 2.0)
      (Class|NavModifierComponent|SetAreaClass (Variables|Default|GetNavModifier)))))

(event EventBeginPlay
  (Utilities|SetHeadColor))

(fn ConstructionScript)

(fn FNWorkFind
  (bind _outactors (Actor|GetAllActorsOfClass "/Game/Buildings/BP_Industry.BP_Industry_C"))
  (if (Utilities|Array|IsEmpty _outactors)
    _
    (else
      (Utilities|IsValid (Utilities|Array|Get(acopy) _outactors (Math|Random|RandomInteger (Utilities|Array|Length _outactors)))
        (:Is%20Valid
          (bind _output_get (Variables|Default|SetWork (Utilities|Array|Get(acopy) _outactors (Math|Random|RandomInteger (Utilities|Array|Length _outactors)))))
          (Variables|Default|SetWork%20Location (Transformation|GetActorLocation _output_get))
          (return))
        (:Is%20Not%20Valid
          _))))
  (Actor|DestroyActor))