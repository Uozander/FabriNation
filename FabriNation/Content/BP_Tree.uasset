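; BP_Tree is a tree actor that snaps itself onto the surface found by a trace when play begins.
; BeginPlay line-traces from its location along an offset vector, ignoring train stations, and moves to the hit point.
; It destroys itself if it hits a river spline or nothing.
; A separate GenerateTree graph, not called here, waits briefly, then spawns another tree at a random positive X/Y offset.
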(event EventBeginPlay
  (bind _returnvalue (Transformation|GetActorLocation))
  (bind _outactors (Actor|GetAllActorsOfClass "/Game/BP_TrainStation.BP_TrainStation_C"))
  (bind (_outhit _returnvalue_2) (Collision|LineTraceForObjects _returnvalue (+ _returnvalue (Variables|Default|GetVector)) (Variables|Default|GetObject%20Types) false _outactors "None" true "(R=1.000000,G=0.000000,B=0.000000,A=1.000000)" "(R=0.000000,G=1.000000,B=0.000000,A=1.000000)" 1.0))
  (if _returnvalue_2
    (if (== (Utilities|GetClass (.hitactor _outhit)) "/Game/LevelPrototyping/Materials/BP_SplineRiver.BP_SplineRiver_C")
      (Actor|DestroyActor :!label _label)
      (else
        (Transformation|SetActorLocation (.location _outhit) false false)))
    (else
      (Development|PrintString (Utilities|String|ToString(Boolean) _returnvalue_2))
      (goto _label))))

(fn ConstructionScript)