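; BP_Building is a building actor that guards against overlapping placement and spawns homes for citizens.
; Shortly after BeginPlay, it destroys itself if it overlaps another exact-class BP_Building whose Structure material is not MAT_Trans.
; CE_HomeSpawn line traces toward one of four random fixed offsets from Structure.
; If clear, it spawns a BP_Residential there and sets the citizen's HomeLocation, with no retry when blocked.
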(event Custom|CE_HomeSpawn
  (params (Citizen :type Actor%20Object%20Reference))
  (bind _structure (Variables|Default|GetStructure))
  (bind _structure_2 (Variables|Default|GetStructure))
  (bind _structure_3 (Variables|Default|GetStructure))
  (bind _structure_4 (Variables|Default|GetStructure))
  (bind _returnvalue (Transformation|GetWorldLocation _structure_2))
  (bind _returnvalue_2 (Transformation|GetWorldLocation _structure_3))
  (bind _returnvalue_3 (Transformation|GetWorldLocation _structure_4))
  (bind _returnvalue_4 (Transformation|GetWorldLocation _structure))
  (bind _returnvalue_5 (+ _returnvalue_4 "250.000000,-250.000000,0.000000"))
  (bind _returnvalue_6 (+ _returnvalue "250.000000,0.000000,0.000000"))
  (bind _returnvalue_7 (+ _returnvalue_2 "-250.000000,0.000000,0.000000"))
  (bind _returnvalue_8 (+ _returnvalue_3 "250.000000,250.000000,0.000000"))
  (switch int (Math|Random|RandomInteger 4)
    (:0
      (bind _returnvalue_9 (Collision|LineTraceByChannel _returnvalue _returnvalue_6 "TraceTypeQuery1" false 0 "None"))
      (if (not _returnvalue_9)
        (Game|SpawnActorfromClass "/Game/BP_Residential.BP_Residential_C" (Math|Transform|MakeTransform _returnvalue_6 "0, 0, 0" "1.000000,1.000000,1.000000") "Undefined" "MultiplyWithRoot" 0 0)
        (bind _asbp_citizen (Utilities|Casting|CastToBP_Citizen Citizen))
        (Variables|/Game/BP_Citizen.BP_Citizen_C|SetHome%20Location _asbp_citizen _returnvalue_6)))
    (:1
      (bind (_outhit _returnvalue_10) (Collision|LineTraceByChannel _returnvalue_2 _returnvalue_7 "TraceTypeQuery1" false 0 "None"))
      (if (not _returnvalue_10)
        (Game|SpawnActorfromClass "/Game/BP_Residential.BP_Residential_C" (Math|Transform|MakeTransform _returnvalue_7 "0, 0, 0" "1.000000,1.000000,1.000000") "Undefined" "MultiplyWithRoot" 0 0)
        (bind _asbp_citizen_2 (Utilities|Casting|CastToBP_Citizen Citizen))
        (Variables|/Game/BP_Citizen.BP_Citizen_C|SetHome%20Location _asbp_citizen_2 _returnvalue_7)))
    (:2
      (bind _returnvalue_11 (Collision|LineTraceByChannel _returnvalue_3 _returnvalue_8 "TraceTypeQuery1" false 0 "None"))
      (if (not _returnvalue_11)
        (Game|SpawnActorfromClass "/Game/BP_Residential.BP_Residential_C" (Math|Transform|MakeTransform _returnvalue_8 "0, 0, 0" "1.000000,1.000000,1.000000") "Undefined" "MultiplyWithRoot" 0 0)
        (bind _asbp_citizen_3 (Utilities|Casting|CastToBP_Citizen Citizen))
        (Variables|/Game/BP_Citizen.BP_Citizen_C|SetHome%20Location _asbp_citizen_3 _returnvalue_8)))
    (:3
      (bind _returnvalue_12 (Collision|LineTraceByChannel _returnvalue_4 _returnvalue_5 "TraceTypeQuery1" false 0 "None"))
      (if (not _returnvalue_12)
        (Game|SpawnActorfromClass "/Game/BP_Residential.BP_Residential_C" (Math|Transform|MakeTransform _returnvalue_5 "0, 0, 0" "1.000000,1.000000,1.000000") "Undefined" "MultiplyWithRoot" 0 0)
        (bind _asbp_citizen_4 (Utilities|Casting|CastToBP_Citizen Citizen))
        (Variables|/Game/BP_Citizen.BP_Citizen_C|SetHome%20Location _asbp_citizen_4 _returnvalue_5)))))

(event EventBeginPlay
  (bind _overlappingactors (Collision|GetOverlappingActors "BP_Building_C" :!class /Script/Engine.Actor))
  (Utilities|FlowControl|Delay 0.1)
  (if (not (Utilities|Array|IsEmpty _overlappingactors))
    (Utilities|IsValid (Variables|Default|GetBox)
      (:Is%20Valid
        (for _array_element _overlappingactors
          (if (== (Utilities|GetClass _array_element) "BP_Building_C")
            (bind _asbp_building (Utilities|Casting|CastToBP_Building _array_element))
            (Utilities|IsValid (Variables|BP_Building_C|GetStructure _asbp_building)
              (:Is%20Valid
                (if (not (== (Rendering|Material|GetMaterial (Variables|BP_Building_C|GetStructure _asbp_building) 0) "/Game/MAT_Trans.MAT_Trans"))
                  (Actor|DestroyActor))))))))))

(fn ConstructionScript)