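; BP_Residential is a housing building that houses citizens and grows in tiers, removing itself shortly after spawning if it overlaps BP_Industry.
; CE_TierUp sets the citizen's home, raises Level, notifies their workplace and reveals another hidden structure mesh, or destroys the citizen at the level cap.
; CE_HomeSpawn line-traces one random cardinal direction and, if clear, spawns an adjacent BP_Residential as the citizen's home, also raising this building's Level.
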(event Custom|CE_HomeSpawn
  (params (Citizen :type Actor%20Object%20Reference))
  (Variables|Default|SetCitizen Citizen)
  (switch int (Math|Random|RandomInteger 4)
    (:0
      (CallFunction|SpawnHome (Variables|Default|GetCitizen) (Variables|Default|GetNorth)))
    (:1
      (CallFunction|SpawnHome (Variables|Default|GetCitizen) (Variables|Default|GetSouth)))
    (:2
      (CallFunction|SpawnHome (Variables|Default|GetCitizen) (Variables|Default|GetWest)))
    (:3
      (CallFunction|SpawnHome (Variables|Default|GetCitizen) (Variables|Default|GetEast)))))

(event Custom|CE_TierUp
  (params (Citizen :type Actor%20Object%20Reference))
  (if (>= (Variables|Default|GetLevel) 5)
    (Actor|DestroyActor Citizen)
    (else
      (bind _asbp_citizen (Utilities|Casting|CastToBP_Citizen Citizen))
      (Variables|/Game/BP_Citizen.BP_Citizen_C|SetHome%20Location _asbp_citizen (Transformation|GetActorLocation))
      (bind _output_get (Variables|Default|SetLevel (+ (Variables|Default|GetLevel) 1)))
      (Default|CEWorkerUP (Variables|/Game/BP_Citizen.BP_Citizen_C|GetWork _asbp_citizen))
      (switch int _output_get
        (:1
          (Rendering|SetVisibility (Variables|Default|GetStructure1) true true))
        (:2
          (Rendering|SetVisibility (Variables|Default|GetBase_Structure1) true true))
        (:3
          (Rendering|SetVisibility (Variables|Default|GetBase_Structure2) true true))
        (:4
          (Rendering|SetVisibility (Variables|Default|GetBase_Structure3) true true))))))

(event EventBeginPlay
  (bind _overlappingactors (Collision|GetOverlappingActors "/Game/BP_Industry.BP_Industry_C" :!class /Script/Engine.Actor))
  (Rendering|SetVisibility (Variables|Default|GetStructure1) false true)
  (Utilities|FlowControl|Delay 0.1)
  (if (not (Utilities|Array|IsEmpty _overlappingactors))
    (Utilities|IsValid (Variables|Default|GetBox)
      (:Is%20Valid
        (for _array_element _overlappingactors
          (if (== (Utilities|GetClass _array_element) "/Game/BP_Industry.BP_Industry_C")
            (Actor|DestroyActor)))))))

(fn ConstructionScript)

(fn SpawnHome
  (params (Object :type Actor%20Object%20Reference) (Direction :type Vector))
  (bind _structure_0 (Variables|Default|GetStructure-0))
  (bind _returnvalue (Transformation|GetWorldLocation _structure_0))
  (bind _returnvalue_2 (+ _returnvalue Direction))
  (bind _returnvalue_3 (Collision|LineTraceByChannel _returnvalue _returnvalue_2 "TraceTypeQuery1" false 0 "None"))
  (if (not _returnvalue_3)
    (Game|SpawnActorfromClass "BP_Residential_C" (Math|Transform|MakeTransform _returnvalue_2 "0, 0, 0" "1.000000,1.000000,1.000000") "Undefined" "MultiplyWithRoot" 0 0)
    (Variables|Default|SetLevel (+ (Variables|Default|GetLevel) 1))
    (bind _asbp_citizen (Utilities|Casting|CastToBP_Citizen Object))
    (Variables|/Game/BP_Citizen.BP_Citizen_C|SetHome%20Location _asbp_citizen _returnvalue_2)
    (return)))