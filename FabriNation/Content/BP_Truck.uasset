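; BP_Truck is a one-shot delivery vehicle that carries a Delivery from where it stands to a target building, then destroys itself.
; CE_Deliver branches on OreNumber: 0 goes to the last BP_TrainStation found, 1 to a BP_Industry picked with a random bias toward lower CoalOre.
; Timelines lerp its location, with play rate set from distance and Speed, then hand the Delivery over on finish.
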(event Custom|CE_Deliver
  (params (Delivery :type STCT%20Resource%20Structure))
  (switch int (.Ore_Number (Utilities|Struct|BreakSTCT_Resource Delivery))
    (:0
      (Variables|Default|SetWork%20Location (Transformation|GetActorLocation))
      (bind _outactors (Actor|GetAllActorsOfClass "/Game/BP_TrainStation.BP_TrainStation_C"))
      (if (Utilities|Array|IsEmpty _outactors)
        (Actor|DestroyActor)
        (else
          (for _array_element _outactors
            (bind _output_get (Variables|Default|SetTrainStation _array_element)))
          (Variables|Default|SetDelivery%20Location (Transformation|GetActorLocation _output_get))
          (Components|Timeline|SetPlayRate (Variables|Default|GetTimeline_0) (/ 1.0 (/ (Math|Vector|Distance(Vector) (Variables|Default|GetWork%20Location) (Variables|Default|GetDelivery%20Location)) (Variables|Default|GetSpeed))))
          (bind _newtrack_0 (Timeline|Timeline PlayFromStart)
            (:Update
              (Transformation|SetActorLocation (Math|Vector|Lerp(Vector) (Variables|Default|GetWork%20Location) (Variables|Default|GetDelivery%20Location) _newtrack_0) false false))
            (:Finished
              (Default|CEDelivery (Variables|Default|GetTrainStation) Delivery)
              (Actor|DestroyActor))))))
    (:1
      (Variables|Default|SetWork%20Location (Transformation|GetActorLocation))
      (bind _outactors_2 (Actor|GetAllActorsOfClass "/Game/BP_Industry.BP_Industry_C"))
      (if (Utilities|Array|IsEmpty _outactors_2)
        (Actor|DestroyActor)
        (else
          (for _array_element_2 _outactors_2
            (if (Utilities|IsValid (Variables|Default|GetDelivery%20Target))
              (if (< (Variables|/Game/BP_Industry.BP_Industry_C|GetCoal%20Ore _array_element_2) (Variables|/Game/BP_Industry.BP_Industry_C|GetCoal%20Ore (Variables|Default|GetDelivery%20Target)))
                (if (>= (- (Math|Random|RandomFloat) (/ (Variables|/Game/BP_Industry.BP_Industry_C|GetCoal%20Ore _array_element_2) 2000)) 0.5)
                  (Variables|Default|SetDelivery%20Target _array_element_2)))
              (else
                (Variables|Default|SetDelivery%20Target _array_element_2))))
          (Variables|Default|SetDelivery%20Location (Transformation|GetActorLocation (Variables|Default|GetDelivery%20Target)))
          (Components|Timeline|SetPlayRate (Variables|Default|GetTimeline_0) (/ 1.0 (/ (Math|Vector|Distance(Vector) (Variables|Default|GetWork%20Location) (Variables|Default|GetDelivery%20Location)) (Variables|Default|GetSpeed))))
          (bind _newtrack_0_2 (Timeline|Timeline_0 PlayFromStart)
            (:Update
              (Transformation|SetActorLocation (Math|Vector|Lerp(Vector) (Variables|Default|GetWork%20Location) (Variables|Default|GetDelivery%20Location) _newtrack_0_2) false false))
            (:Finished
              (Default|CEDeliver (Variables|Default|GetDelivery%20Target) Delivery)
              (Actor|DestroyActor))))))))

(fn ConstructionScript)